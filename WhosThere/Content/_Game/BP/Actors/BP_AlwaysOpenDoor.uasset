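; BP_AlwaysOpenDoor is an interactable door actor that swings its mesh open and closed with no lock or condition.
; Interact prints a debug string, triggers the OpenDoor event and returns the door's static mesh.
; OpenDoor uses a FlipFlop to alternately play and reverse a timeline that lerps the mesh's relative yaw between closed and open.
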(event Custom|OpenDoor
  (Utilities|FlowControl|FlipFlop
    (:A
      (bind _newtrack_0 (Timeline|TL_ChangeDoorStatus Play)
        (:Update
          (Transformation|SetRelativeRotation (Variables|Default|GetMesh) (Math|Rotator|MakeRotator 0.0 0.0 (Math|Float|Lerp 0.0 1.1e+02 _newtrack_0)) false false))))
    (:B
      (Timeline|TL_ChangeDoorStatus Reverse))))

(fn ConstructionScript)

(fn Interact
  (Development|PrintString "interact")
  (CallFunction|OpenDoor)
  (return (Variables|/Script/Engine.StaticMeshComponent|GetStaticMesh (Variables|Default|GetMesh))))