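; BP_NextLvlKey is a key pickup actor that notifies a linked Door when the player collects it, apparently for level progression.
; Interact prints a debug string, triggers HideItem and returns the key's static mesh to the caller.
; HideItem calls PickupKeyMessage on the Door, then destroys the actor after a short delay.
; An alternative hide-and-disable-collision branch is left unconnected.
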(event Custom|HideItem
  (Class|BPIDoorInteract|PickupKey(Message) (Variables|Default|GetDoor))
  (Utilities|FlowControl|Delay 0.2)
  (Actor|DestroyActor))

(fn ConstructionScript)

(fn Interact
  (Development|PrintString "interact")
  (CallFunction|HideItem)
  (return (Variables|/Script/Engine.StaticMeshComponent|GetStaticMesh (Variables|Default|GetMesh))))