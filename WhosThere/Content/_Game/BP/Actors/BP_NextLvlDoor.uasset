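; BP_NextLvlDoor is an interactable, key-locked door that leads to the next level.
; Interact calls OpenDoor, which toggles a timeline that swings the mesh open or closed once PickupKey has set HasKey.
; Without the key, it briefly shows a door-locked widget.
; A trigger overlap by the first-person character plays a fade transition widget, then loads Lvl_WhosThere_Start after a short delay.
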(event OnComponentBeginOverlap(NextLvlTrigger)
  (params (OverlappedComponent :type Primitive%20Component%20Object%20Reference) (OtherActor :type Actor%20Object%20Reference) (OtherComp :type Primitive%20Component%20Object%20Reference) (OtherBodyIndex :type Integer) (bFromSweep :type Boolean) (SweepResult :type Hit%20Result%20Structure%20%28by%20ref%29))
  (Utilities|Casting|CastToBP_FirstPersonCharacter OtherActor)
  (bind _returnvalue (UserInterface|CreateWidget "/Game/_Game/UI/WBP_Transition.WBP_Transition_C"))
  (UserInterface|Viewport|AddtoViewport _returnvalue 0)
  (Default|FadeAnimation _returnvalue)
  (Utilities|FlowControl|Delay 1.0)
  (Game|OpenLevel(byName) "Lvl_WhosThere_Start"))

(event Custom|OpenDoor
  (if (Variables|Default|GethasKey?)
    (Utilities|FlowControl|FlipFlop
      (:A
        (bind _newtrack_0 (Timeline|TL_ChangeDoorStatus Play)
          (:Update
            (Transformation|SetRelativeRotation (Variables|Default|GetMesh) (Math|Rotator|MakeRotator 0.0 0.0 (Math|Float|Lerp 0.0 1.1e+02 _newtrack_0)) false false))))
      (:B
        (Timeline|TL_ChangeDoorStatus Reverse)))
    (else
      (bind _asbp_first_person_player_controller (Utilities|Casting|CastToBP_FirstPersonPlayerController (Game|GetPlayerController 0)))
      (bind _returnvalue (UserInterface|CreateWidget "/Game/_Game/UI/WBP_DoorLocked.WBP_DoorLocked_C" _asbp_first_person_player_controller))
      (UserInterface|Viewport|AddtoViewport _returnvalue 0)
      (Utilities|FlowControl|Delay 1.0)
      (Widget|RemovefromParent _returnvalue))))

(event EventPickupKey
  (Variables|Default|SethasKey? true))

(fn ConstructionScript)

(fn Interact
  (Development|PrintString "interact")
  (CallFunction|OpenDoor)
  (return (Variables|/Script/Engine.StaticMeshComponent|GetStaticMesh (Variables|Default|GetMesh))))