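; BP_MasterNote is a note actor, apparently a base for other notes, that the first-person player can interact with to read.
; Interact triggers PickupNote and returns the static mesh of its Cube component to the caller.
; PickupNote flags HasNote on BP_FirstPersonCharacter, adds a WBP_MasterNote widget to the viewport, shows the mouse cursor and pauses the game.
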(event Custom|PickupNote
  (bind _returnvalue (Game|GetPlayerController 0))
  (bind _asbp_first_person_character (Utilities|Casting|CastToBP_FirstPersonCharacter (Game|GetPlayerCharacter 0)))
  (Variables|/Game/FirstPerson/Blueprints/BP_FirstPersonCharacter.BP_FirstPersonCharacter_C|SethasNote? _asbp_first_person_character true)
  (bind _returnvalue_2 (UserInterface|CreateWidget "/Game/_Game/UI/Notes/WBP_MasterNote.WBP_MasterNote_C" _returnvalue))
  (UserInterface|Viewport|AddtoViewport _returnvalue_2 0)
  (Variables|/Script/Engine.PlayerController|SetbShowMouseCursor _returnvalue true)
  (Game|SetGamePaused true))

(event EventBeginPlay)

(event Collision|EventActorBeginOverlap
  (params (OtherActor :type Actor%20Object%20Reference)))

(event EventTick
  (params (DeltaSeconds :type Float%20%28single-precision%29)))

(fn ConstructionScript)

(fn Interact
  (CallFunction|PickupNote)
  (return (Variables|/Script/Engine.StaticMeshComponent|GetStaticMesh (Variables|Default|GetCube))))