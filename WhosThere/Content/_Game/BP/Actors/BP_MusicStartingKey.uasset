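; BP_MusicStartingKey is an interactable key pickup that triggers a music change when collected.
; Interact fires HideItem and returns the key's static mesh, and HideItem sends a pickup message to its referenced Door.
; If the BP_Door found by class lookup has the key, the game instance fades into radio static, then after a delay into a music track.
; The actor then destroys itself.
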(event Custom|HideItem
  (bind _returnvalue (Game|GetGameInstance))
  (Class|BPIDoorInteract|PickupKey(Message) (Variables|Default|GetDoor))
  (bind _returnvalue_2 (Actor|GetActorOfClass "/Game/_Game/BP/Actors/BP_Door.BP_Door_C"))
  (if (Variables|/Game/_Game/BP/Actors/BP_Door.BP_Door_C|GethasKey? _returnvalue_2)
    (Class|BPIMusicPlayer|PlayMusic(Message) _returnvalue 3.0 0.0 "/Game/_Game/FX/SFX/SFX_radio-static-industrial-sfx_Cue.SFX_radio-static-industrial-sfx_Cue")
    (Utilities|FlowControl|Delay 4.0)
    (Class|BPIMusicPlayer|PlayMusic(Message) _returnvalue 0.0 1.0 "/Game/_Game/FX/SFX/Music/SFX_bensound-theuninvited_Cue.SFX_bensound-theuninvited_Cue")
    (Utilities|FlowControl|Delay 0.2)
    (Actor|DestroyActor)))

(fn ConstructionScript)

(fn Interact
  (Development|PrintString "interact")
  (CallFunction|HideItem)
  (return (Variables|/Script/Engine.StaticMeshComponent|GetStaticMesh (Variables|Default|GetMesh))))