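; BP_CameraFocusTrigger is a one-shot box trigger that turns the first-person player's view toward a static mesh.
; On the first overlap by BP_FirstPersonCharacter it shows the mesh and plays the FocusCamera timeline.
; Each timeline update interpolates from the character's actor rotation toward the mesh and applies it as control rotation.
; A delay started from that update hides the mesh again a few seconds later.
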(event OnComponentBeginOverlap(Box)
  (params (OverlappedComponent :type Primitive%20Component%20Object%20Reference) (OtherActor :type Actor%20Object%20Reference) (OtherComp :type Primitive%20Component%20Object%20Reference) (OtherBodyIndex :type Integer) (bFromSweep :type Boolean) (SweepResult :type Hit%20Result%20Structure%20%28by%20ref%29))
  (bind _staticmesh (Variables|Default|GetStaticMesh))
  (bind _staticmesh_2 (Variables|Default|GetStaticMesh))
  (bind _returnvalue (Transformation|GetWorldLocation _staticmesh))
  (bind _asbp_first_person_character (Utilities|Casting|CastToBP_FirstPersonCharacter OtherActor))
  (Utilities|FlowControl|DoOnce false
    (:Completed
      (Rendering|SetVisibility _staticmesh_2 true false)
      (Timeline|FocusCamera Play
        (:Update
          (Pawn|SetControlRotation (Game|GetPlayerController 0) (Math|Interpolation|RInterpTo (Transformation|GetActorRotation _asbp_first_person_character) (Math|Rotator|FindLookatRotation (Transformation|GetActorLocation _asbp_first_person_character) (Math|Vector|MakeVector (.x _returnvalue) (.y _returnvalue) (.z _returnvalue))) (Utilities|Time|GetWorldDeltaSeconds) 2.0))
          (Utilities|FlowControl|Delay 5.0)
          (Rendering|SetVisibility _staticmesh_2 false false))))))

(event EventBeginPlay)

(event Collision|EventActorBeginOverlap
  (params (OtherActor :type Actor%20Object%20Reference)))

(event EventTick
  (params (DeltaSeconds :type Float%20%28single-precision%29)))

(fn ConstructionScript)