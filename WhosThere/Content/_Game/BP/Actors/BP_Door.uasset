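; Door actor that swings open and closed on interaction once its HasKey flag is set by PickupKey.
; Interact calls OpenDoor and returns the door's static mesh.
; With the key, a FlipFlop plays or reverses a timeline that lerps the mesh yaw between closed and open.
; Without it, a locked-door widget shows briefly while player input is disabled.
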(event Custom|OpenDoor
  (bind _returnvalue (Game|GetPlayerController 0))
  (if (Variables|Default|GethasKey?)
    (Utilities|FlowControl|FlipFlop
      (:A
        (bind _newtrack_0 (Timeline|TL_ChangeDoorStatus Play)
          (:Update
            (Transformation|SetRelativeRotation (Variables|Default|GetMesh) (Math|Rotator|MakeRotator 0.0 0.0 (Math|Float|Lerp 0.0 1.1e+02 _newtrack_0)) false false))))
      (:B
        (Timeline|TL_ChangeDoorStatus Reverse)))
    (else
      (bind _asbp_first_person_player_controller (Utilities|Casting|CastToBP_FirstPersonPlayerController (Game|GetPlayerController 0)))
      (bind _returnvalue_2 (UserInterface|CreateWidget "/Game/_Game/UI/WBP_DoorLocked.WBP_DoorLocked_C" _asbp_first_person_player_controller))
      (UserInterface|Viewport|AddtoViewport _returnvalue_2 0)
      (Input|DisableInput _returnvalue 0)
      (Utilities|FlowControl|Delay 1.0)
      (Widget|RemovefromParent _returnvalue_2)
      (Input|EnableInput _returnvalue 0))))

(event EventPickupKey
  (Variables|Default|SethasKey? true))

(fn ConstructionScript)

(fn Interact
  (Development|PrintString "interact")
  (CallFunction|OpenDoor)
  (return (Variables|/Script/Engine.StaticMeshComponent|GetStaticMesh (Variables|Default|GetMesh))))