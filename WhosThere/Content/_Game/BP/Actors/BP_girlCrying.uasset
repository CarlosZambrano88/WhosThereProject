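; BP_girlCrying is an actor that plays a scare sequence when the first-person character overlaps its Trigger component.
; The overlap plays a static girl-talking sound, then a scream after a short delay.
; It then adds a WBP_Static widget to the player controller's viewport and removes it after a long timed delay.
; The trigger has no once-only guard and is never disabled.
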(event OnComponentBeginOverlap(Trigger)
  (params (OverlappedComponent :type Primitive%20Component%20Object%20Reference) (OtherActor :type Actor%20Object%20Reference) (OtherComp :type Primitive%20Component%20Object%20Reference) (OtherBodyIndex :type Integer) (bFromSweep :type Boolean) (SweepResult :type Hit%20Result%20Structure%20%28by%20ref%29))
  (Utilities|Casting|CastToBP_FirstPersonCharacter OtherActor)
  (Audio|PlaySound2D (Variables|Default|GetStaticGirlTalkingTrigger) 1.5 1.0 0.0 0 0)
  (Utilities|FlowControl|Delay 0.25)
  (Audio|PlaySound2D (Variables|Default|GetgirlScreamingSFX) 1.5 1.0 0.0 0 0)
  (bind _asbp_first_person_player_controller (Utilities|Casting|CastToBP_FirstPersonPlayerController (Game|GetPlayerController 0)))
  (bind _returnvalue (UserInterface|CreateWidget "/Game/_Game/UI/WBP_Static.WBP_Static_C" _asbp_first_person_player_controller))
  (UserInterface|Viewport|AddtoViewport _returnvalue 0)
  (Utilities|FlowControl|Delay 26.0)
  (Widget|RemovefromParent _returnvalue))

(event EventBeginPlay)

(event Collision|EventActorBeginOverlap
  (params (OtherActor :type Actor%20Object%20Reference)))

(event EventTick
  (params (DeltaSeconds :type Float%20%28single-precision%29)))

(fn ConstructionScript)